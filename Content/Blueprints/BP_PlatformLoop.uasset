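; BP_PlatformLoop is a moving platform meant to either loop or move on demand, selected by PlatformBehavior.
; In loop mode, Timeline_0 drives PlatformTimelineUpdate, re-entering the delayed Play until the mesh exactly reaches EndLocation, then reverses after a delay (TODO flags a long wait).
; On-demand mode uses Box overlaps and a second Timeline: end overlap reverses it, but a constant-false branch blocks Play on begin overlap.
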(event `self.ReceiveBeginPlay`
  ;[1 1 1] "Loop" action. TODO: fix long delay before reverse
  (if (== (`self.PlatformBehavior`) 1)
    (`KismetSystemLibrary.Delay` 3.0 :!label _label)
    (bind (_direction _platform_alpha) (`Timeline|Timeline_0` :!label _label_2)
      (:`Update`
        (`self.PlatformTimelineUpdate` _platform_alpha)
        (bind _output_get (set `self.CurrentLocation` (`SceneComponent.RelativeLocation` (`self.PlatformMesh`))))
        (if (== (`self.EndLocation`) _output_get)
          (`KismetSystemLibrary.Delay` 1.5)
          (goto _label_2 :!via `Reverse`)
          (else
            (goto _label)))))
    (else
      ;[1 1 1] "On demand" action
      ;;[1 1 1] BeginPlay signal stopper
      (if false
        (if false :!label _label_3
          (bind (_direction_2 _platform_alpha_2) (`Timeline|Timeline` :!label _label_4)
            (:`Update`
              (`self.PlatformTimelineUpdate` _platform_alpha_2))))))))

(event `self.Box.OnComponentBeginOverlap`
  (params (OverlappedComponent :type "PrimitiveComponent Object Reference") (OtherActor :type "Actor Object Reference") (OtherComp :type "PrimitiveComponent Object Reference") (OtherBodyIndex :type Integer) (bFromSweep :type Boolean) (SweepResult :type "HitResult Structure (by ref)"))
  ;[1 1 1] "On demand" action
  (goto _label_3))

(event `self.Box.OnComponentEndOverlap`
  (params (OverlappedComponent :type "PrimitiveComponent Object Reference") (OtherActor :type "Actor Object Reference") (OtherComp :type "PrimitiveComponent Object Reference") (OtherBodyIndex :type Integer))
  ;[1 1 1] "On demand" action
  (goto _label_4 :!via `Reverse`))

(fn `UserConstructionScript`)