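; Player character Blueprint that changes the camera spring arm length while the player sprints.
; BeginPlay caches the default arm length, and the sprint start and end events extend the parent class's behavior.
; A timeline plays on sprint start to interpolate the arm toward the sprint length, then reverses on sprint end to ease it back.
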(event `self.ReceiveBeginPlay`
  (set `self.DefaultArmLength` (`SpringArmComponent.TargetArmLength` (`self.SpringArmComponent`))))

(event `self.OnSprintStart`
  (`parent.OnSprintStart`)
  (bind (_direction _newtrack_0) (`Timeline|SpringArmSprintTimeline` :!label _label)
    (:`Update`
      (set `SpringArmComponent.TargetArmLength` (`KismetMathLibrary.Lerp` (`self.DefaultArmLength`) (`self.SprintArmLength`) _newtrack_0) (`self.SpringArmComponent`)))))

(event `self.OnSprintEnd`
  (`parent.OnSprintEnd`)
  (goto _label :!via `Reverse`))

(fn `UserConstructionScript`)