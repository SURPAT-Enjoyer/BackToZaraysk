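; BP_Player is the player character Blueprint, which routes strafe-related input to a StrafeComponent.
; Enhanced Input actions for A, D and Space pass their pressed and released states to the component's handler functions.
; The A and D events also set IsAPressed and IsDPressed flags on the player.
; BeginPlay runs the "show collision" console command, toggling the collision debug view.
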(event `EnhancedInput|/Game/BackToZaraysk/Core/Input/Actions/Strafe/IA_D`
  (params (ActionValue :type Boolean) (ElapsedSeconds :type "Float (double-precision)") (TriggeredSeconds :type "Float (double-precision)") (InputAction :type "InputAction Object Reference" :default "/Game/BackToZaraysk/Core/Input/Actions/Strafe/IA_D.IA_D"))
  (:`Started`
    (`StrafeComponent.HandleDInput` (`self.StrafeComponent`) true)
    (set `self.bIsDPressed` true)))

(event `EnhancedInput|/Game/BackToZaraysk/Core/Input/Actions/Strafe/IA_Space`
  (params (ActionValue :type Boolean) (ElapsedSeconds :type "Float (double-precision)") (TriggeredSeconds :type "Float (double-precision)") (InputAction :type "InputAction Object Reference" :default "/Game/BackToZaraysk/Core/Input/Actions/Strafe/IA_Space.IA_Space"))
  (:`Started`
    (`StrafeComponent.HandleSpaceInput` (`self.StrafeComponent`) true)))

(event `EnhancedInput|/Game/BackToZaraysk/Core/Input/Actions/Strafe/IA_D`
  (params (ActionValue :type Boolean) (ElapsedSeconds :type "Float (double-precision)") (TriggeredSeconds :type "Float (double-precision)") (InputAction :type "InputAction Object Reference" :default "/Game/BackToZaraysk/Core/Input/Actions/Strafe/IA_D.IA_D"))
  (:`Completed`
    (`StrafeComponent.HandleDInput` (`self.StrafeComponent`) false)
    (set `self.bIsDPressed` false)))

(event `EnhancedInput|/Game/BackToZaraysk/Core/Input/Actions/Strafe/IA_A`
  (params (ActionValue :type Boolean) (ElapsedSeconds :type "Float (double-precision)") (TriggeredSeconds :type "Float (double-precision)") (InputAction :type "InputAction Object Reference" :default "/Game/BackToZaraysk/Core/Input/Actions/Strafe/IA_A.IA_A"))
  (:`Started`
    (`StrafeComponent.HandleAInput` (`self.StrafeComponent`) true)
    (set `self.bIsAPressed` true)))

(event `EnhancedInput|/Game/BackToZaraysk/Core/Input/Actions/Strafe/IA_Space`
  (params (ActionValue :type Boolean) (ElapsedSeconds :type "Float (double-precision)") (TriggeredSeconds :type "Float (double-precision)") (InputAction :type "InputAction Object Reference" :default "/Game/BackToZaraysk/Core/Input/Actions/Strafe/IA_Space.IA_Space"))
  (:`Completed`
    (`StrafeComponent.HandleSpaceInput` (`self.StrafeComponent`) false)))

(event `EnhancedInput|/Game/BackToZaraysk/Core/Input/Actions/Strafe/IA_A`
  (params (ActionValue :type Boolean) (ElapsedSeconds :type "Float (double-precision)") (TriggeredSeconds :type "Float (double-precision)") (InputAction :type "InputAction Object Reference" :default "/Game/BackToZaraysk/Core/Input/Actions/Strafe/IA_A.IA_A"))
  (:`Completed`
    (`StrafeComponent.HandleAInput` (`self.StrafeComponent`) false)
    (set `self.bIsAPressed` false)))

(event `self.ReceiveBeginPlay`
  (`KismetSystemLibrary.ExecuteConsoleCommand` "show collision" null))

(fn `UserConstructionScript`)