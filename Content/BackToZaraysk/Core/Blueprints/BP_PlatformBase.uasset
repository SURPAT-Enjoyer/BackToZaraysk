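; BP_PlatformBase is a moving-platform Blueprint that animates its motion with timelines.
; While PlatformBehavior equals 1, Tick plays a timeline whose alpha feeds PlatformTimelineUpdate, which is defined outside this graph.
; EventReverse reverses that timeline, while leaving BoxCollision reverses PlatformMovement_Timeline through the same update function.
; Begin-overlap and timer-elapsed events are empty, and the timer setup and ReverseEndLocation assignment are disconnected.
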(event `self.ReceiveTick`
  (params (DeltaSeconds :type "Float (single-precision)"))
  (if (== (`self.PlatformBehavior`) 1)
    (bind (_direction _platform_alpha) (`Timeline|Timeline` :!label _label)
      (:`Update`
        (`self.PlatformTimelineUpdate` _platform_alpha)))))

(event `EventReverse`
  (params (DeltaSeconds :type "Float (single-precision)"))
  (goto _label :!via `Reverse`))

(event `self.BoxCollision.OnComponentBeginOverlap`
  (params (OverlappedComponent :type "PrimitiveComponent Object Reference") (OtherActor :type "Actor Object Reference") (OtherComp :type "PrimitiveComponent Object Reference") (OtherBodyIndex :type Integer) (bFromSweep :type Boolean) (SweepResult :type "HitResult Structure (by ref)")))

(event `OnPlatformTimerElapsed`)

(event `self.BoxCollision.OnComponentEndOverlap`
  (params (OverlappedComponent :type "PrimitiveComponent Object Reference") (OtherActor :type "Actor Object Reference") (OtherComp :type "PrimitiveComponent Object Reference") (OtherBodyIndex :type Integer))
  (`|ExecutionSequence`
    (:`then_1`
      (bind (_direction _platform_alpha) (`Timeline|PlatformMovement_Timeline` :!via `Reverse`)
        (:`Update`
          (`self.PlatformTimelineUpdate` _platform_alpha))))))

(fn `UserConstructionScript`)